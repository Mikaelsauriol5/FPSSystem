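; FPSCharacter is an AI-driven pawn that chases pawns it sees and can be killed by projectiles.
; Its PawnSensing component triggers a simple move toward each seen pawn through the pawn's own controller.
; Overlapping a Bullet_Projectile prints a hit message and subtracts fixed damage from Health, destroying the actor once Health is depleted.
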(event OnSeePawn(PawnSensing)
  (params (Pawn :type Pawn%20Object%20Reference))
  (AI|Navigation|SimpleMovetoActor (Pawn|GetController) Pawn))

(event EventBeginPlay)

(event Collision|EventActorBeginOverlap
  (params (OtherActor :type Actor%20Object%20Reference))
  (Utilities|Casting|CastToBullet_Projectile OtherActor)
  (Development|PrintString "Hit")
  (Variables|Default|SetHealth (- (Variables|Default|GetHealth) 10))
  (if (<= (Variables|Default|GetHealth) 0)
    (Actor|DestroyActor)))

(event EventTick
  (params (DeltaSeconds :type Float%20%28single-precision%29)))

(fn ConstructionScript)