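; Pistol ammo pickup actor that adds reserve ammo to the player's weapon and then disappears.
; On BeginPlay the ammo mesh simulates physics for one second to settle, then physics turns off.
; When Player_BP overlaps the collision, inventory slot 1's MaxAmmo rises by that weapon's magazine size.
; It then plays a pickup sound at its location and destroys itself.
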(event OnComponentBeginOverlap(Collision)
  (params (OverlappedComponent :type Primitive%20Component%20Object%20Reference) (OtherActor :type Actor%20Object%20Reference) (OtherComp :type Primitive%20Component%20Object%20Reference) (OtherBodyIndex :type Integer) (bFromSweep :type Boolean) (SweepResult :type Hit%20Result%20Structure%20%28by%20ref%29))
  (bind _asplayer_bp (Utilities|Casting|CastToPlayer_BP OtherActor))
  (Utilities|Struct|SetmembersinWeapon_Struct (Variables|/Game/FPS_System/Game/Blueprints/Weapon_BP.Weapon_BP_C|GetWeaponData (Utilities|Array|Get(acopy) (Variables|/Game/FPS_System/Game/Blueprints/Player_BP.Player_BP_C|GetWeaponInventory _asplayer_bp) 1)) (+ (.MaxAmmo (Utilities|Struct|BreakWeapon_Struct (Variables|/Game/FPS_System/Game/Blueprints/Weapon_BP.Weapon_BP_C|GetWeaponData (Utilities|Array|Get(acopy) (Variables|/Game/FPS_System/Game/Blueprints/Player_BP.Player_BP_C|GetWeaponInventory _asplayer_bp) 1)))) (.MagazineSize (Utilities|Struct|BreakWeapon_Struct (Variables|/Game/FPS_System/Game/Blueprints/Weapon_BP.Weapon_BP_C|GetWeaponData (Utilities|Array|Get(acopy) (Variables|/Game/FPS_System/Game/Blueprints/Player_BP.Player_BP_C|GetWeaponInventory _asplayer_bp) 1))))))
  (Audio|PlaySoundatLocation "/Game/FPS_System/Game/Sounds/Wave/AmmoPickup.AmmoPickup" (Transformation|GetActorLocation))
  (Actor|DestroyActor))

(event EventBeginPlay
  (bind _ammo (Variables|Default|GetAmmo))
  (Physics|SetSimulatePhysics _ammo true)
  (Utilities|FlowControl|Delay 1.0)
  (Physics|SetSimulatePhysics _ammo false))

(fn ConstructionScript)