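; Behavior tree task that picks a random wander destination for an AI-controlled FPS_Character.
; After a short random delay, it casts to AiController1 and its pawn, then turns sprinting off.
; It writes a random reachable point within a radius of the controller actor's location to the DestLocation blackboard key and finishes successfully.
; It does no movement itself, and a failed cast leaves the task unfinished.
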(event EventReceiveExecute
  (params (OwnerActor :type Actor%20Object%20Reference))
  (Utilities|FlowControl|Delay (Math|Random|RandomFloatinRange 0.0 3.0))
  (bind _asai_controller_1 (Utilities|Casting|CastToAiController1 OwnerActor))
  (bind _asfps_character (Utilities|Casting|CastToFPS_Character (Pawn|GetControlledPawn _asai_controller_1)))
  (Variables|/Game/FPS_System/Game/Blueprints/FPS_Character.FPS_Character_C|SetisSprinting _asfps_character false)
  (AI|BehaviorTree|SetBlackboardValueasVector (Variables|Default|GetdestLocation) (.RandomLocation (AI|Navigation|GetRandomReachablePointinRadius (Transformation|GetActorLocation OwnerActor) 3e+03)))
  (AI|BehaviorTree|FinishExecute true))